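; BP_RunnableWall is a wall actor that tells overlapping actors when they can wall-run along it and in which direction.
; Two trigger components, C1 and C2, each send SetRunableWallMessage on begin overlap, passing their own transform as the start point and the other component's location as the target, so either can be the start.
; Leaving either trigger sends a disable message with a zero target.
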(event `self.c1.OnComponentBeginOverlap`
  (params (OverlappedComponent :type "PrimitiveComponent Object Reference") (OtherActor :type "Actor Object Reference") (OtherComp :type "PrimitiveComponent Object Reference") (OtherBodyIndex :type Integer) (bFromSweep :type Boolean) (SweepResult :type "HitResult Structure (by ref)"))
  (message `/Game/Shared_Blueprints/_Connor_Blueprints/Grapple/BPI_Wallrunner.SetRunableWall` OtherActor true (`SceneComponent.K2_GetComponentLocation` (`self.c2`)) (`SceneComponent.K2_GetComponentToWorld` (`self.c1`))))

(event `self.c1.OnComponentEndOverlap`
  (params (OverlappedComponent :type "PrimitiveComponent Object Reference") (OtherActor :type "Actor Object Reference") (OtherComp :type "PrimitiveComponent Object Reference") (OtherBodyIndex :type Integer))
  (message `/Game/Shared_Blueprints/_Connor_Blueprints/Grapple/BPI_Wallrunner.SetRunableWall` OtherActor false (0.0 0.0 0.0) (struct)))

(event `self.c2.OnComponentBeginOverlap`
  (params (OverlappedComponent :type "PrimitiveComponent Object Reference") (OtherActor :type "Actor Object Reference") (OtherComp :type "PrimitiveComponent Object Reference") (OtherBodyIndex :type Integer) (bFromSweep :type Boolean) (SweepResult :type "HitResult Structure (by ref)"))
  (message `/Game/Shared_Blueprints/_Connor_Blueprints/Grapple/BPI_Wallrunner.SetRunableWall` OtherActor true (`SceneComponent.K2_GetComponentLocation` (`self.c1`)) (`SceneComponent.K2_GetComponentToWorld` (`self.c2`))))

(event `self.c2.OnComponentEndOverlap`
  (params (OverlappedComponent :type "PrimitiveComponent Object Reference") (OtherActor :type "Actor Object Reference") (OtherComp :type "PrimitiveComponent Object Reference") (OtherBodyIndex :type Integer))
  (message `/Game/Shared_Blueprints/_Connor_Blueprints/Grapple/BPI_Wallrunner.SetRunableWall` OtherActor false (0.0 0.0 0.0) (struct)))

(fn `UserConstructionScript`)