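; Collectable Earth pickup that the third-person character collects by pressing E while inside its box collision.
; Overlap begin and end toggle the actor's input and add or remove an interact prompt widget.
; Pressing E briefly sets the prompt's pressed flag, decrements the game mode's remaining-collectables count, shows a collectable widget and destroys the actor.
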(event `Key|E`
  (params (Key :type "Key Structure"))
  (:`Pressed`
    (set `/Game/Shared_Assets/AbbyAssets/Collectables/Interact_Prompt_Widget.IsPressed` true (stale `self.Box Collison.OnComponentBeginOverlap` _returnvalue))
    (`KismetSystemLibrary.Delay` 0.3)
    (set `/Game/Shared_Assets/AbbyAssets/Collectables/Interact_Prompt_Widget.IsPressed` false (stale `self.Box Collison.OnComponentBeginOverlap` _returnvalue))))

(event `Key|E`
  (params (Key :type "Key Structure"))
  (:`Pressed`
    (bind _ascollectable_game_mode (cast `/Game/Shared_Assets/COllectable_gamemode/Collectable_Game_Mode` (`GameplayStatics.GetGameMode`)))
    (bind _result (`/Engine/EditorBlueprintResources/StandardMacros.DecrementInt` (`/Game/Shared_Assets/COllectable_gamemode/Collectable_Game_Mode.Collectables Left` _ascollectable_game_mode))
      (:`  `
        (set `/Game/Shared_Assets/COllectable_gamemode/Collectable_Game_Mode.Collectables Left` _result _ascollectable_game_mode)
        (bind _returnvalue (`|CreateWidget` "/Game/Shared_Assets/AbbyAssets/Collectables/Collectable_widget.Collectable_widget_C"))
        (`UserWidget.AddToViewport` _returnvalue 0)
        (`self.K2_DestroyActor`)))))

(event `self.Box Collison.OnComponentBeginOverlap`
  (params (OverlappedComponent :type "PrimitiveComponent Object Reference") (OtherActor :type "Actor Object Reference") (OtherComp :type "PrimitiveComponent Object Reference") (OtherBodyIndex :type Integer) (bFromSweep :type Boolean) (SweepResult :type "HitResult Structure (by ref)"))
  (cast `/Game/Shared_Blueprints/Chacracter/ThirdPersonCharacter` OtherActor)
  (`self.EnableInput` (`GameplayStatics.GetPlayerController` 0))
  (bind _returnvalue (`|CreateWidget` "/Game/Shared_Assets/AbbyAssets/Collectables/Interact_Prompt_Widget.Interact_Prompt_Widget_C"))
  (`UserWidget.AddToViewport` _returnvalue 0))

(event `self.Box Collison.OnComponentEndOverlap`
  (params (OverlappedComponent :type "PrimitiveComponent Object Reference") (OtherActor :type "Actor Object Reference") (OtherComp :type "PrimitiveComponent Object Reference") (OtherBodyIndex :type Integer))
  (cast `/Game/Shared_Blueprints/Chacracter/ThirdPersonCharacter` OtherActor)
  (`self.DisableInput` (`GameplayStatics.GetPlayerController` 0))
  (`Widget.RemoveFromParent` (stale `self.Box Collison.OnComponentBeginOverlap` _returnvalue)))

(fn `UserConstructionScript`)